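; BP_Basket is a player-controlled basket that moves sideways in response to Enhanced Input.
; BeginPlay stores its Box in the Platform variable and adds the IMC_Default mapping context to the first player controller's input subsystem.
; IA_Move passes its X value to Move, which applies forced movement input along the right vector of the control rotation's yaw and roll, ignoring pitch.
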(event Input|EnhancedActionEvents|EnhancedInputActionIA_Move
  (params (ActionValue :type Vector%202D%20Structure) (ElapsedSeconds :type Float%20%28double-precision%29) (TriggeredSeconds :type Float%20%28double-precision%29) (InputAction :type Input%20Action%20Object%20Reference :default "/Game/Input/Actions/IA_Move.IA_Move"))
  (CallFunction|Move (.x ActionValue)))

(event EventBeginPlay
  (Variables|Default|SetPlatform (Variables|Default|GetBox))
  (CallFunction|SetInput))

(fn ConstructionScript)

(fn SetInput
  (bind _asplayer_controller (Utilities|Casting|CastToPlayerController (Game|GetPlayerController 0)))
  (Utilities|IsValid (PlayerController|LocalPlayerSubsystems|GetEnhancedInputLocalPlayerSubsystem _asplayer_controller)
    (:Is%20Valid
      (Input|AddMappingContext (PlayerController|LocalPlayerSubsystems|GetEnhancedInputLocalPlayerSubsystem _asplayer_controller) "/Game/Input/IMC_Default.IMC_Default" 0 "(bIgnoreAllPressedKeysUntilRelease=True,bForceImmediately=False,bNotifyUserSettings=False)"))))

(fn Move
  (params (Direction :type Float%20%28double-precision%29))
  (bind _returnvalue (Pawn|GetControlRotation :!class /Script/Engine.Pawn))
  (Pawn|Input|AddMovementInput (Math|Vector|GetRightVector (Math|Rotator|MakeRotator (.roll _returnvalue) 0.0 (.yaw _returnvalue))) Direction true))
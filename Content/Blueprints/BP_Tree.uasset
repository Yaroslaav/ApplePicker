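; BP_Tree is a moving tree that slides sideways and spawns apples as it goes.
; Each tick runs a countdown that spawns a BPApple at a random point along Y around the tree, then re-rolls the delay up to SpawnRate.
; Movement input follows the control rotation's right vector, with direction forced inward outside the Y bounds and randomly flipped at 1-in-16 odds per tick inside them.
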(event EventBeginPlay
  (Variables|Default|SetTimeToSpawn (Variables|Default|GetSpawnRate)))

(event EventTick
  (params (DeltaSeconds :type Float%20%28single-precision%29))
  (CallFunction|TrySpawnApple DeltaSeconds)
  (CallFunction|TryChangeDirection)
  (CallFunction|Move))

(fn ConstructionScript)

(fn SpawnApple
  (bind _returnvalue (Game|SpawnActorfromClass (Variables|Default|GetBP_Apple) (Math|Transform|MakeTransform (Math|Random|RandomPointinBoundingBox (Transformation|GetActorLocation) (Math|Vector|MakeVector 0.0 (Variables|Default|GetSpawningAreaHalfSize) 0.0))) "AdjustIfPossibleButAlwaysSpawn" "MultiplyWithRoot" 0 0))
  (Variables|Default|SetTimeToSpawn (Math|Random|RandomFloatinRange 0.5 (Variables|Default|GetSpawnRate)))
  (return _returnvalue))

(fn TrySpawnApple
  (params (DeltaTime :type Float%20%28double-precision%29))
  (bind _output_get (Variables|Default|SetTimeToSpawn (- (Variables|Default|GetTimeToSpawn) DeltaTime)))
  (if (<= _output_get 0.0)
    (CallFunction|SpawnApple)))

(fn TryChangeDirection
  (bind _inbounds (CallFunction|CheckBounds))
  (if _inbounds
    (if (== 15 (Math|Random|RandomInteger 16))
      (Variables|Default|SetMoveDirection (* -1.0 (Variables|Default|GetMoveDirection))))))

(fn Move
  (bind _returnvalue (Pawn|GetControlRotation :!class /Script/Engine.Pawn))
  (Pawn|Input|AddMovementInput (Math|Vector|GetRightVector (Math|Rotator|MakeRotator (.roll _returnvalue) 0.0 (.yaw _returnvalue))) (Variables|Default|GetMoveDirection) true))

(fn CheckBounds
  (bind _defaultsceneroot (Variables|Default|GetDefaultSceneRoot))
  (bind _moveybounds (Variables|Default|GetMoveYBounds))
  (bind _returnvalue (Transformation|GetWorldLocation _defaultsceneroot))
  (if (< (.y _returnvalue) (.x _moveybounds))
    (Variables|Default|SetMoveDirection 1.0)
    (elif (> (.y _returnvalue) (.y _moveybounds))
      (Variables|Default|SetMoveDirection -1.0)
      (else
        (return true))))
  (return false))